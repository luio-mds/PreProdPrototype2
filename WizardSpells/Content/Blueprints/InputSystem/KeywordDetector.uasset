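; KeywordDetector is an input Blueprint for typing incantations, captured key by key from raw input.
; Enter toggles a KeywordInputWindow widget and the detection flag, printing the incantation text on close.
; While detecting, Any Key uses key display names to append characters or handle Backspace and Space Bar, updating the widget's text.
; Single characters pass through CheckLetterCase, whose Shift-based case selection appears unconnected.
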(event `Key|Enter`
  (params (Key :type "Key Structure"))
  (bind _inputwindow (`self.InputWindow`))
  (:`Pressed`
    (`/Engine/EditorBlueprintResources/StandardMacros.IsValid` _inputwindow
      (:`Is Valid`
        (`Widget.RemoveFromParent` _inputwindow)
        (set `self.InputWindow` null)
        (`KismetSystemLibrary.PrintString` (`self.CurrentIncantationText`))
        (set `self.DetectingKeystroke` false)
        (`KismetSystemLibrary.PrintString` "Finished Incantation"))
      (:`Is Not Valid`
        (bind _returnvalue (`|CreateWidget` "/Game/Blueprints/InputSystem/KeywordInputWindow.KeywordInputWindow_C"))
        (bind _output_get (set `self.InputWindow` _returnvalue))
        (`UserWidget.AddToViewport` _output_get 0)
        (`KismetSystemLibrary.PrintString` "Entering Incantation...")
        (set `self.DetectingKeystroke` true)))))

(event `Key|AnyKey`
  (params (Key :type "Key Structure"))
  (bind _returnvalue (`KismetTextLibrary.Conv_TextToString` (`KismetInputLibrary.Key_GetDisplayName` Key)))
  (bind _displaytextbox (`/Game/Blueprints/InputSystem/KeywordInputWindow.DisplayTextBox` (`self.InputWindow`)))
  (bind _returnvalue_2 (`KismetTextLibrary.Conv_TextToString` (`TextBlock.Text` _displaytextbox)))
  (:`Pressed`
    (if (`self.DetectingKeystroke`)
      (if (> (`KismetStringLibrary.Len` _returnvalue) 1)
        (switch `string` _returnvalue
          (:`Space Bar`
            (bind _output_get (set `self.CurrentIncantationText` (`KismetStringLibrary.Concat_StrStr` _returnvalue_2 " ")))
            (set `TextBlock.Text` (`KismetTextLibrary.Conv_StringToText` _output_get) _displaytextbox))
          (:`BACKSPACE`
            (bind _output_get_2 (set `self.CurrentIncantationText` (`KismetStringLibrary.LeftChop` _returnvalue_2 1)))
            (set `TextBlock.Text` (`KismetTextLibrary.Conv_StringToText` _output_get_2) _displaytextbox)))
        (else
          (bind _output_get_3 (set `self.CurrentIncantationText` (`KismetStringLibrary.Concat_StrStr` _returnvalue_2 (`self.CheckLetterCase` _returnvalue))))
          (set `TextBlock.Text` (`KismetTextLibrary.Conv_StringToText` _output_get_3) _displaytextbox))))))

(fn `UserConstructionScript`)
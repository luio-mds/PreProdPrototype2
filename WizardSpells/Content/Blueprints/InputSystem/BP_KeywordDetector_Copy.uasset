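; Keyword detector for typed spellcasting: Enter toggles an incantation window that slows time and drains player mana on a timer.
; Keystrokes build the incantation and refresh a mana cost preview from keyword multipliers.
; Keywords are validated by position against DT_Keywords and unlock state: base spell last, element before it, modifiers earlier.
; Submitting broadcasts the assembled spell with multiplied stats or signals failure, then updates the current spell widget.
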(event `self.ReceiveBeginPlay`
  (`|ExecutionSequence`
    (:`then_0`
      (bind _returnvalue (`|CreateWidget` "/Game/UI/WBP_CurrentSpell.WBP_CurrentSpell_C"))
      (bind _output_get (set `self.CurrentSpellWidget` _returnvalue))
      (`UserWidget.AddToViewport` _output_get 0)
      (`WidgetBlueprintLibrary.SetInputMode_GameAndUIEx` (`GameplayStatics.GetPlayerController` 0) null)
      (bind _asbp_top_down_character (cast `/Game/TopDown/Blueprints/BP_TopDownCharacter` (`GameplayStatics.GetPlayerCharacter` 0)))
      (set `self.As BP Top Down Character` _asbp_top_down_character))))

(event `DisplayManaCost`
  (bind _manacostmultiplier (`self.ManaCostMultiplier`))
  (bind _manacostmultiplier_2 (`self.ManaCostMultiplier`))
  (bind _manacostmultiplier_3 (`self.ManaCostMultiplier`))
  (bind _manacostmultiplier_4 (`self.ManaCostMultiplier`))
  (bind (_final_spell_condition_basespell _final_spell_condition_element _final_spell_condition_modifier) (break `/Game/Blueprints/InputSystem/ST_FinalSpellCondition` (`self.Final Spell Condition`)))
  (bind (_wordname _wordtype _description _damagemultiplier _manacostmultiplier_5) (break `/Game/Blueprints/InputSystem/ST_KeywordData` (`self.Modifier`)))
  (bind (_wordname_2 _wordtype_2 _description_2 _damagemultiplier_2 _manacostmultiplier_6) (break `/Game/Blueprints/InputSystem/ST_KeywordData` (`self.Basespell`)))
  (bind (_wordname_3 _wordtype_3 _description_3 _damagemultiplier_3 _manacostmultiplier_7) (break `/Game/Blueprints/InputSystem/ST_KeywordData` (`self.Element`)))
  (bind _manacosttext (`/Game/Blueprints/InputSystem/BP_KeywordInputWindow.ManaCostText` (`self.InputWindow`)))
  ; total mana cost
  (set `self.PlenishRestoration` 0.0)
  (set `self.ManaCostMultiplier` 0.0)
  (`self.SeparateKeywords` (`self.CurrentIncantationText`)
    (:`Out`
      (`self.ValidateKeywords`
        (:`Found`
          (if _final_spell_condition_basespell
            (set `self.ManaCostMultiplier` (`KismetMathLibrary.SelectFloat` _manacostmultiplier_6 (* _manacostmultiplier_3 _manacostmultiplier_6) (== _manacostmultiplier_3 0.0))))
          (if _final_spell_condition_element
            (set `self.ManaCostMultiplier` (`KismetMathLibrary.SelectFloat` _manacostmultiplier_7 (* _manacostmultiplier_4 _manacostmultiplier_7) (== _manacostmultiplier_4 0.0))))
          (if _final_spell_condition_modifier
            (bind _output_get (set `self.ManaCostMultiplier` (`KismetMathLibrary.SelectFloat` _manacostmultiplier_5 (* _manacostmultiplier _manacostmultiplier_5) (== _manacostmultiplier 0.0)))))
          (`KismetSystemLibrary.PrintString` (`KismetStringLibrary.Conv_DoubleToString` _output_get))
          (if (== _manacostmultiplier_2 0.0)
            (`TextBlock.SetText` _manacosttext "0")
            (else
              (`TextBlock.SetText` _manacosttext (`KismetTextLibrary.Conv_DoubleToText` (* _manacostmultiplier_2 1.0) "HalfToEven")))))))))

(event `Key|Enter`
  (params (Key :type "Key Structure"))
  (bind _returnvalue (`GameplayStatics.GetPlayerCameraManager` 0))
  (bind _inputwindow (`self.InputWindow`))
  ;[0.54 1 0 0.5] Input window
  (:`Pressed`
    (`/Engine/EditorBlueprintResources/StandardMacros.IsValid` _inputwindow
      (:`Is Valid`
        (`Widget.RemoveFromParent` _inputwindow)
        (set `self.InputWindow` null)
        (`KismetSystemLibrary.PrintString` (`self.CurrentIncantationText`))
        (set `self.DetectingKeystroke` false)
        (`GameplayStatics.SetGlobalTimeDilation` 1.0)
        (`self.StopMPDrain`)
        (`Widget.RemoveFromParent` (`self.InputMaskWidget`))
        (`self.SeparateKeywords` (`self.CurrentIncantationText`)
          (:`Out`
            (bind _spell_condition (`self.ValidateKeywords`)
              (:`Found`
                (bind _composedspell (`self.AssembleSpell` (`self.Modifier`) (`self.Element`) (`self.Basespell`) (`.Modifier_7_464EB0114D50B10CB740969DF875F370` (break `/Game/Blueprints/InputSystem/ST_FinalSpellCondition` _spell_condition))))
                (`self.OnSpellCast` _composedspell)
                ;[1 0 0.2015 0.5] debug
                (`PlayerCameraManager.StartCameraFade` _returnvalue 0.0 1.0 0.1 (struct :`R` 0.562196 :`G` 1.0 :`A` 1.0) false false))
              (:`Not Found`
                ;[1 0.2956 0 0.5] Can put failed spells effect / damage here
                (`KismetSystemLibrary.PrintString` "invalid incantation" true true (struct :`R` 1.0 :`B` 0.172637 :`A` 1.0))
                (`PlayerCameraManager.StartCameraFade` _returnvalue 0.0 1.0 0.1 (struct :`R` 1.0 :`G` 0.009688 :`B` 4.1e-05 :`A` 1.0) false false)
                (`GameplayStatics.PlaySound2D` "/Game/Audio/Ouch_Test_Cue.Ouch_Test_Cue" 0.5 1.0 0.8 null null)))
            (`self.DisplayCurrentSpell` (`self.Final Spell Condition`) (`self.CurrentSpellWidget`)))))
      (:`Is Not Valid`
        (bind _returnvalue_2 (`|CreateWidget` "/Game/Blueprints/InputSystem/BP_KeywordInputWindow.BP_KeywordInputWindow_C"))
        (bind _output_get (set `self.InputWindow` _returnvalue_2))
        (`UserWidget.AddToViewport` _output_get 0)
        (set `self.DetectingKeystroke` true)
        (`self.ResetOnStartTyping`)
        ; Jandre Code
        (`GameplayStatics.SetGlobalTimeDilation` (`self.Time Dilation`))
        ;[1 0.5739 0 0.5] MP Drain Timer
        (bind _returnvalue_3 (`KismetSystemLibrary.K2_SetTimerDelegate` (delegate `ReducePlayerMP`) (`self.Time Dilation`) true))
        (set `self.MPTimer` _returnvalue_3)
        (`self.ReducePlayerMP`) ; First frame reduction
        (bind _returnvalue_4 (`|CreateWidget` "/Game/UI/WBP_InputMask.WBP_InputMask_C"))
        (bind _output_get_2 (set `self.InputMaskWidget` _returnvalue_4))
        (`UserWidget.AddToViewport` _output_get_2 -1))))
  (:`Released`
    (bind _foundwidgets (`WidgetBlueprintLibrary.GetAllWidgetsOfClass` "/Game/UI/WBP_Tutorial.WBP_Tutorial_C"))
    (for _array_element _foundwidgets
      (if (`Widget.IsVisible` (`/Game/UI/WBP_Tutorial.EnterText` _array_element))
        (`/Game/UI/WBP_Tutorial.EnterClicked` _array_element)))))

(event `ReducePlayerMP`
  (bind _as_bp_top_down_character (`self.As BP Top Down Character`))
  ;[1 0.5739 0 0.5] MP Drain Timer
  (bind _output_get (set `/Game/TopDown/Blueprints/BP_TopDownCharacter.PlayerMana` (`KismetMathLibrary.FClamp` (- (`/Game/TopDown/Blueprints/BP_TopDownCharacter.PlayerMana` _as_bp_top_down_character) (`self.ManaReduceRate`)) 0.0 100.0) _as_bp_top_down_character))
  ;[1 0 0.1124 0.5] debug
  (`KismetSystemLibrary.PrintString` (`KismetStringLibrary.Concat_StrStr` "Current Mana: " (`KismetStringLibrary.Conv_DoubleToString` _output_get))))

(event `StopMPDrain`
  ;[1 0.5739 0 0.5] MP Drain Timer
  (`KismetSystemLibrary.K2_PauseTimerHandle` (`self.MPTimer`)))

(event `Key|AnyKey`
  (params (Key :type "Key Structure"))
  (bind _returnvalue (`KismetTextLibrary.Conv_TextToString` (`KismetInputLibrary.Key_GetDisplayName` Key)))
  (bind _displaytextbox (`/Game/Blueprints/InputSystem/BP_KeywordInputWindow.DisplayTextBox` (`self.InputWindow`)))
  (bind _returnvalue_2 (`KismetTextLibrary.Conv_TextToString` (`TextBlock.Text` _displaytextbox)))
  ;[0.4113 1 0 0.5] Key Detection
  (:`Pressed`
    (if (`self.DetectingKeystroke`)
      (if (> (`KismetStringLibrary.Len` _returnvalue) 1)
        (switch `string` _returnvalue
          (:`Space Bar`
            (bind _output_get (set `self.CurrentIncantationText` (`KismetStringLibrary.Concat_StrStr` _returnvalue_2 " ")))
            (set `TextBlock.Text` (`KismetTextLibrary.Conv_StringToText` _output_get) _displaytextbox))
          (:`BACKSPACE`
            (bind _output_get_2 (set `self.CurrentIncantationText` (`KismetStringLibrary.LeftChop` _returnvalue_2 1)))
            (set `TextBlock.Text` (`KismetTextLibrary.Conv_StringToText` _output_get_2) _displaytextbox)))
        (else
          (bind _output_get_3 (set `self.CurrentIncantationText` (`KismetStringLibrary.Concat_StrStr` _returnvalue_2 (`self.CheckLetterCase` _returnvalue))))
          (set `TextBlock.Text` (`KismetTextLibrary.Conv_StringToText` _output_get_3) _displaytextbox)))
      (`self.DisplayManaCost`))))

(event `ResetOnStartTyping`
  ;[1 1 1 0.5] reset stuff
  (set `self.CurrentIncantationText` "")
  (`KismetArrayLibrary.Array_Clear` (`self.DetectedKeywords`))
  (set `self.BasespellKeyword` "")
  (set `self.ElementKeyword` "")
  (`KismetArrayLibrary.Array_Clear` (`self.ModifierKeywords`))
  (`KismetArrayLibrary.Array_Clear` (`self.UniqueKeywords`))
  (set `self.Final Spell Condition` (make `/Game/Blueprints/InputSystem/ST_FinalSpellCondition` false))
  (set `self.Basespell` (struct))
  (set `self.Element` (struct))
  (set `self.Modifier` (struct)))

(fn `AssembleSpell`
  (params (ModifierRow :type "/Game/Blueprints/InputSystem/ST_KeywordData Structure") (ElementRow :type "/Game/Blueprints/InputSystem/ST_KeywordData Structure") (BasespellRow :type "/Game/Blueprints/InputSystem/ST_KeywordData Structure") (bHasModifier :type Boolean))
  (returns (ComposedSpell :type "/Game/Blueprints/InputSystem/ST_ComposedSpell Structure"))
  (bind (_wordname _wordtype _description _damagemultiplier _manacostmultiplier _sizemultiplier) (break `/Game/Blueprints/InputSystem/ST_KeywordData` ModifierRow))
  (bind (_wordname_2 _wordtype_2 _description_2 _damagemultiplier_2 _manacostmultiplier_2 _sizemultiplier_2) (break `/Game/Blueprints/InputSystem/ST_KeywordData` ElementRow))
  (bind (_wordname_3 _wordtype_3 _description_3 _damagemultiplier_3 _manacostmultiplier_3 _sizemultiplier_3) (break `/Game/Blueprints/InputSystem/ST_KeywordData` BasespellRow))
  (return (make `/Game/Blueprints/InputSystem/ST_ComposedSpell` (`KismetStringLibrary.Concat_StrStr` (`KismetStringLibrary.Conv_NameToString` _wordname) " \" \"" (`KismetStringLibrary.Conv_NameToString` _wordname_2) " \" \"" (`KismetStringLibrary.Conv_NameToString` _wordname_3)) (* (* (`KismetMathLibrary.SelectFloat` _damagemultiplier 1.0 bHasModifier) _damagemultiplier_2) _damagemultiplier_3) (* (* (`KismetMathLibrary.SelectFloat` _manacostmultiplier 1.0 bHasModifier) _manacostmultiplier_2) _manacostmultiplier_3) (* (* (`KismetMathLibrary.SelectFloat` _sizemultiplier 1.0 bHasModifier) _sizemultiplier_2) _sizemultiplier_3) ModifierRow ElementRow BasespellRow)))

(fn `DisplayCurrentSpell`
  (params (condition :type "/Game/Blueprints/InputSystem/ST_FinalSpellCondition Structure") (widget :type "/Game/UI/WBP_CurrentSpell Object Reference"))
  (bind (_basespell _element _modifier) (break `/Game/Blueprints/InputSystem/ST_FinalSpellCondition` condition))
  (bind (_modifier_wordname _modifier_wordtype _modifier_description) (break `/Game/Blueprints/InputSystem/ST_KeywordData` (`self.Modifier`)))
  (bind (_basespell_wordname _basespell_wordtype _basespell_description) (break `/Game/Blueprints/InputSystem/ST_KeywordData` (`self.Basespell`)))
  (bind (_element_wordname _element_wordtype _element_description) (break `/Game/Blueprints/InputSystem/ST_KeywordData` (`self.Element`)))
  (`TextBlock.SetText` (`/Game/UI/WBP_CurrentSpell.ModifierText` widget) (`KismetMathLibrary.SelectText` (`KismetTextLibrary.Conv_NameToText` _modifier_wordname) "" _modifier))
  (`TextBlock.SetText` (`/Game/UI/WBP_CurrentSpell.ModifierDescriptionText` widget) (`KismetMathLibrary.SelectText` _modifier_description "" _modifier))
  (`TextBlock.SetText` (`/Game/UI/WBP_CurrentSpell.ElementText` widget) (`KismetMathLibrary.SelectText` (`KismetTextLibrary.Conv_NameToText` _element_wordname) "" _element))
  (`TextBlock.SetText` (`/Game/UI/WBP_CurrentSpell.ElementDescriptionText` widget) (`KismetMathLibrary.SelectText` _element_description "" _element))
  (`TextBlock.SetText` (`/Game/UI/WBP_CurrentSpell.BasespellText` widget) (`KismetMathLibrary.SelectText` (`KismetTextLibrary.Conv_NameToText` _basespell_wordname) "" _basespell))
  (`TextBlock.SetText` (`/Game/UI/WBP_CurrentSpell.BasespellDescriptionText` widget) (`KismetMathLibrary.SelectText` _basespell_description "" _basespell)))

(fn `UserConstructionScript`)
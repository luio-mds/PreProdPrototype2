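; BC_Statistics measures the player's typing speed, stored as WPM on the BP_TopDownCharacter pawn it caches at BeginPlay.
; CalculateWPM checks BP_KeywordDetector: while keystroke detection is on it records a start time, otherwise it divides SpellsTyped by the elapsed time.
; The result is effectively spells per second, as the divide-by-60 node is unused.
; Debug strings print each state and the computed value.
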(event `self.ReceiveBeginPlay`
  (bind _asbp_top_down_character (cast `/Game/TopDown/Blueprints/BP_TopDownCharacter` (`GameplayStatics.GetPlayerPawn` 0)))
  (set `self.As BP Top Down Character` _asbp_top_down_character))

(event `CalculateWPM`
  (bind _as_bp_top_down_character (`self.As BP Top Down Character`))
  (bind _returnvalue (`GameplayStatics.GetActorOfClass` "/Game/Blueprints/InputSystem/BP_KeywordDetector.BP_KeywordDetector_C"))
  (if (`/Game/Blueprints/InputSystem/BP_KeywordDetector.DetectingKeystroke` _returnvalue)
    (bind _output_get (set `self.StartTime` (`KismetSystemLibrary.GetGameTimeInSeconds`)))
    (`KismetSystemLibrary.PrintString` "start watching wpm")
    (else
      (`KismetSystemLibrary.PrintString` "stop watching wpm")
      (bind _output_get_2 (set `self.TimeElapsed` (- (`KismetSystemLibrary.GetGameTimeInSeconds`) _output_get)))
      (bind _output_get_3 (set `/Game/TopDown/Blueprints/BP_TopDownCharacter.WPM` (`KismetMathLibrary.Conv_IntToDouble` (/ (`/Game/TopDown/Blueprints/BP_TopDownCharacter.SpellsTyped` _as_bp_top_down_character) _output_get_2)) _as_bp_top_down_character))
      (`KismetSystemLibrary.PrintString` (`KismetStringLibrary.Concat_StrStr` "WPM: " (`KismetStringLibrary.Conv_DoubleToString` _output_get_3))))))